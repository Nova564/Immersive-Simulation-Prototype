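; BP_TrainVehicle is a player-controlled train that rides along TrackManager's main or bis spline and creates a HUD linked to itself.
; Keys set target speed to full, stop or hold, and toggle the bis-track choice, applied only within a fixed distance window.
; Each tick eases speed, advances a looping spline distance, places both bogies, then centres and aligns the visual body between them with a sideways offset.
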(event `self.ReceiveBeginPlay`
  (bind _returnvalue (`|CreateWidget` "/Game/Blueprints/UI/WBP_HUD.WBP_HUD_C"))
  (set `/Game/Blueprints/UI/WBP_HUD.MyTrain` self _returnvalue)
  (`UserWidget.AddToViewport` _returnvalue 0))

(event `self.ReceiveTick`
  (params (DeltaSeconds :type "Float (single-precision)"))
  (bind _trackmanager (`self.TrackManager`))
  (bind _trainvisualroot (`self.TrainVisualRoot`))
  (bind _bogie_rear (`self.Bogie_Rear`))
  (bind _bogie_front (`self.Bogie_Front`))
  (bind _returnvalue (`SceneComponent.K2_GetComponentLocation` _bogie_front))
  (bind _returnvalue_2 (`SceneComponent.K2_GetComponentLocation` _bogie_rear))
  (bind _returnvalue_3 (select `bool` (`self.IsOnBisTrack`) :`false` (`/Game/Blueprints/BP_TrackManager.MainTrack` _trackmanager) :`true` (`/Game/Blueprints/BP_TrackManager.BisTrack` _trackmanager)))
  (set `self.CurrentSpeed` (`KismetMathLibrary.FInterpTo_Constant` (`self.CurrentSpeed`) (`self.TargetSpeed`) (`GameplayStatics.GetWorldDeltaSeconds`) (`self.Power`)))
  (if (`KismetMathLibrary.InRange_FloatFloat` (`self.CurrentDistance`) 1600.0 1950.0)
    (set `self.IsOnBisTrack` (`self.WantsToTakeBis`)))
  (set `self.CurrentDistance` (mod (+ (`self.CurrentDistance`) (* (`self.CurrentSpeed`) (`GameplayStatics.GetWorldDeltaSeconds`))) (`SplineComponent.GetSplineLength` _returnvalue_3)))
  (`SceneComponent.K2_SetWorldLocation` _bogie_rear (`SplineComponent.GetLocationAtDistanceAlongSpline` _returnvalue_3 (`self.CurrentDistance`) "World") false false)
  (`SceneComponent.K2_SetWorldLocation` _bogie_front (`SplineComponent.GetLocationAtDistanceAlongSpline` _returnvalue_3 (+ (`self.CurrentDistance`) (`self.BogieOffset`)) "World") false false)
  (`SceneComponent.K2_SetWorldRotation` _trainvisualroot (`KismetMathLibrary.FindLookAtRotation` _returnvalue_2 _returnvalue) false false)
  (`SceneComponent.K2_SetWorldLocation` _trainvisualroot (+ (`KismetMathLibrary.VLerp` _returnvalue_2 _returnvalue 0.5) (* (`self.GetActorRightVector`) -50.0)) false false))

(event `Key|Z`
  (params (Key :type "Key Structure"))
  (:`Pressed`
    (set `self.TargetSpeed` (`self.MaxSpeed`))))

(event `Key|S`
  (params (Key :type "Key Structure"))
  (:`Pressed`
    (set `self.TargetSpeed` 0.0)))

(event `Key|E`
  (params (Key :type "Key Structure"))
  (:`Pressed`
    (set `self.WantsToTakeBis` (not (`self.WantsToTakeBis`)))))

(event `Key|U`
  (params (Key :type "Key Structure"))
  (:`Pressed`
    (set `self.TargetSpeed` (`self.CurrentSpeed`))))

(fn `UserConstructionScript`)