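; Track switch lever actor whose handle shows whether the train wants to take the bis route.
; On BeginPlay it finds and caches the BP_TrainVehicle in the level.
; Every Tick it reads the train's WantsToTakeBis flag and smoothly interpolates the handle's relative rotation toward one of two opposite tilts.
; It only mirrors the train's state and has no input handling of its own.
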(event `self.ReceiveTick`
  (params (DeltaSeconds :type "Float (single-precision)"))
  (`SceneComponent.K2_SetRelativeRotation` (`self.LeverHandle`) (`KismetMathLibrary.RInterpTo` (`SceneComponent.RelativeRotation` (`self.LeverHandle`)) (`KismetMathLibrary.SelectRotator` (struct :`Roll` 45.0) (struct :`Roll` -45.0) (`/Game/Blueprints/BP_TrainVehicle.WantsToTakeBis` (`self.CachedTrain`))) (`GameplayStatics.GetWorldDeltaSeconds`) 5.0) false false))

(event `self.ReceiveBeginPlay`
  (bind _returnvalue (`GameplayStatics.GetActorOfClass` "/Game/Blueprints/BP_TrainVehicle.BP_TrainVehicle_C"))
  (set `self.CachedTrain` _returnvalue))

(fn `UserConstructionScript`)